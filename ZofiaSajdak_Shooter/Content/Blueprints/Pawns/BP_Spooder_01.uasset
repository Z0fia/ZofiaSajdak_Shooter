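; Spider enemy AI character that chases the player, attacks in melee and dies from damage.
; BeginPlay loops AIMoveTo on the player while alive, and Tick halts movement, zeroes rotation and plays an attack montage when in range, resuming on completion.
; DamagePlayer applies the hit but is not called within this Blueprint.
; At zero health it disables movement and collision, increments BP_Soldier_01's kill count, then destroys itself after a delay.
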(event `self.ReceiveBeginPlay`
  (`|AIMoveTo` self (0.0 0.0 0.0) (`GameplayStatics.GetPlayerCharacter` 0) :!label _label
    (:`OnSuccess`
      _)
    (:`OnFail`
      _))
  (if (`self.IsAlive`)
    (`KismetSystemLibrary.Delay` 0.2)
    (goto _label)))

(event `self.ReceiveTick`
  (params (DeltaSeconds :type "Float (single-precision)"))
  (if (`self.CanAttack`)
    (`self.DeactivateMovement`)
    (`|PlayMontage` (`self.Mesh`) "/Game/Characters/Enemy_Great_Spider/Animations/AM_SpooderAttack_01.AM_SpooderAttack_01"
      (:`OnCompleted`
        (`self.ActivateMovement`)))))

(event `self.ReceiveAnyDamage`
  (params (Damage :type "Float (single-precision)") (DamageType :type "DamageType Object Reference") (InstigatedBy :type "Controller Object Reference") (DamageCauser :type "Actor Object Reference"))
  (bind _output_get (`self.DecreaseHealth` Damage))
  (if (== _output_get 0.0)
    (`self.AIDead`)
    (`KismetSystemLibrary.Delay` 3.0)
    (`self.K2_DestroyActor`)))

(fn `ActivateMovement`
  (`ActorComponent.Activate` (`self.CharacterMovement`) false))

(fn `AIDead`
  (set `self.Dead` true)
  (`self.DeactivateMovement`)
  (`self.SetActorEnableCollision` false)
  (bind _asbp_soldier_01 (cast `/Game/Blueprints/Pawns/BP_Soldier_01` (`GameplayStatics.GetPlayerCharacter` 0)))
  (`/Game/Blueprints/Pawns/BP_Soldier_01.IncreaseKills` _asbp_soldier_01))

(fn `CanAttack`
  (returns (ReturnValue :type Boolean))
  (return (and (`self.IsAttackRange`) (not (`self.IsAttacking`)) (`self.IsAlive`))))

(fn `DamagePlayer`
  (if (`self.IsAlive`)
    (`GameplayStatics.ApplyDamage` (`GameplayStatics.GetPlayerCharacter` 0) (`self.Base Damage`))))

(fn `DeactivateMovement`
  (`self.K2_SetActorRotation` (struct))
  (`MovementComponent.StopMovementImmediately` (`self.CharacterMovement`))
  (`ActorComponent.Deactivate` (`self.CharacterMovement`)))

(fn `DecreaseHealth`
  (params (B :type "Float (double-precision)"))
  (returns (Output_Get :type "Float (double-precision)"))
  (bind _output_get (set `self.HP` (`KismetMathLibrary.FClamp` (- (`self.HP`) B) 0.0 100.0)))
  (return _output_get))

(fn `IsAlive`
  (returns (ReturnValue :type Boolean))
  (return (not (`self.Dead`))))

(fn `IsAttacking`
  (returns (ReturnValue :type Boolean))
  (return (`AnimInstance.Montage_IsPlaying` (`SkeletalMeshComponent.GetAnimInstance` (`self.Mesh`)) "/Game/Characters/Enemy_Great_Spider/Animations/AM_SpooderAttack_01.AM_SpooderAttack_01")))

(fn `IsAttackRange`
  (returns (ReturnValue :type Boolean))
  (return (<= (`self.GetDistanceTo` (`GameplayStatics.GetPlayerCharacter` 0)) (`self.AttackRange`))))

(fn `UserConstructionScript`)