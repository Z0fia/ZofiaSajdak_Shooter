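; BP_Soldier_01 is the player soldier pawn, with world-axis movement, automatic rifle fire, health, a kill counter and a HUD widget.
; While alive, it smoothly turns control rotation toward the direction of mouse movement, ignoring movement within a dead zone.
; Firing starts muzzle effects, sound and a looping timer of line traces that damage blocking hits.
; Incoming damage lowers clamped HP and marks the soldier dead at zero.
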(event `self.ReceiveTick`
  (params (DeltaSeconds :type "Float (single-precision)"))
  (if (`self.IsAlive`)
    (`self.UpdatePlayerRotation`)))

(event `InputAction|Fire Weapon`
  (params (Key :type "Key Structure"))
  (:`Pressed`
    (if (`self.IsAlive`)
      (`self.StartFiringWeapon`)))
  (:`Released`
    (`self.StopFiringWeapon`)))

(event `InputAxis|MoveForward`
  (params (AxisValue :type "Float (single-precision)"))
  (if (`self.IsAlive`)
    (`self.AddMovementInput` (1.0 0.0 0.0) AxisValue)))

(event `self.ReceiveBeginPlay`
  (bind _returnvalue (`|CreateWidget` "/Game/UI/W_PlayerHUD.W_PlayerHUD_C" null self))
  (`UserWidget.AddToViewport` _returnvalue 0))

(event `InputAxis|MoveRight`
  (params (AxisValue :type "Float (single-precision)"))
  (if (`self.IsAlive`)
    (`self.AddMovementInput` (0.0 1.0 0.0) AxisValue)))

(event `self.ReceiveAnyDamage`
  (params (Damage :type "Float (single-precision)") (DamageType :type "DamageType Object Reference") (InstigatedBy :type "Controller Object Reference") (DamageCauser :type "Actor Object Reference"))
  (bind _output_get (`self.DecreaseHealth` Damage))
  (if (== _output_get 0.0)
    (set `self.Dead` true)))

(fn `DecreaseHealth`
  (params (B :type "Float (double-precision)"))
  (returns (Output_Get :type "Float (double-precision)"))
  (bind _output_get (set `self.HP` (`KismetMathLibrary.FClamp` (- (`self.HP`) B) 0.0 100.0)))
  (return _output_get))

(fn `GetMouseVelocit`
  (returns (ReturnValue :type "Vector2D Structure"))
  (bind (_deltax _deltay) (`PlayerController.GetInputMouseDelta` (`GameplayStatics.GetPlayerController` 0)))
  (return (/ (`KismetMathLibrary.MakeVector2D` _deltax _deltay) (`GameplayStatics.GetWorldDeltaSeconds`))))

(fn `IncreaseKills`
  (bind _result (`/Engine/EditorBlueprintResources/StandardMacros.IncrementInt` (`self.Kills`))
    (:`  `
      (set `self.Kills` _result))))

(fn `IsAlive`
  (returns (ReturnValue :type Boolean))
  (return (not (`self.Dead`))))

(fn `IsMouseAboveDeadZone`
  (returns (ReturnValue :type Boolean))
  (return (> (`KismetMathLibrary.VSize2D` (`self.GetMouseVelocit`)) (`self.MouseDeadZone`))))

(fn `StartFiringWeapon`
  (`ActorComponent.Activate` (`self.P_AssaultRifle_MF`) false)
  (bind _returnvalue (`GameplayStatics.SpawnSound2D` "/Game/Sounds/Weapon_AssaultRifle/Stereo/RandomFireloop.RandomFireloop" 1.0 1.0 0.0 null))
  (set `self.WeaponFireSound` _returnvalue)
  (`self.WeaponTrace`)
  (`KismetSystemLibrary.K2_SetTimer` null "WeaponTrace" (`self.FireRate`) true))

(fn `StopFiringWeapon`
  (bind _weaponfiresound (`self.WeaponFireSound`))
  (`ActorComponent.Deactivate` (`self.P_AssaultRifle_MF`))
  (`/Engine/EditorBlueprintResources/StandardMacros.IsValid` _weaponfiresound
    (:`Is Valid`
      (`AudioComponent.Stop` _weaponfiresound)
      (`KismetSystemLibrary.K2_ClearTimer` null "WeaponTrace")
      (if (`self.IsAlive`)
        (`GameplayStatics.SpawnSound2D` "/Game/Sounds/Weapon_AssaultRifle/Stereo/GunFireEnd.GunFireEnd" 1.0 1.0 0.0 null)))))

(fn `UpdatePlayerRotation`
  (bind _returnvalue (`GameplayStatics.GetPlayerController` 0))
  (bind (_returnvalue_x _returnvalue_y) (`KismetMathLibrary.BreakVector2D` (`self.GetMouseVelocit`)))
  (if (`self.IsMouseAboveDeadZone`)
    (`Controller.SetControlRotation` _returnvalue (`KismetMathLibrary.RInterpTo` (`Controller.GetControlRotation` _returnvalue) (`KismetMathLibrary.MakeRotator` 0.0 0.0 (`KismetMathLibrary.DegAtan2` _returnvalue_x _returnvalue_y)) (`GameplayStatics.GetWorldDeltaSeconds`) (`self.DeltaTimeMultiply`)))))

(fn `UserConstructionScript`)

(fn `WeaponTrace`
  (bind _returnvalue (`SceneComponent.GetSocketLocation` (`self.Rifle`) "MuzzleFlashSocket"))
  (bind _outhit (`KismetSystemLibrary.LineTraceSingle` :`Start` _returnvalue :`End` (+ _returnvalue (* (`KismetMathLibrary.GetForwardVector` (`self.GetControlRotation`)) (`self.WeaponRange`))) :`TraceChannel` "TraceTypeQuery1" :`DrawDebugType` "ForDuration"))
  (bind (_bblockinghit _binitialoverlap _time _distance _location _impactpoint _normal _impactnormal _physmat _hitactor) (`GameplayStatics.BreakHitResult` _outhit))
  (if _bblockinghit
    (`GameplayStatics.ApplyDamage` _hitactor (`self.Base Damage`))))