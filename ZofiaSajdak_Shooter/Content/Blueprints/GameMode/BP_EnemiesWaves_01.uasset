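; Wave spawner that continuously spawns BP_Spooder_01 enemies in the level.
; Two seconds after BeginPlay, NewWave increments CurrentWave and starts a looping timer on SpawnWave.
; Each tick of that timer spawns one spooder at a random TargetPoint, chosen from all TargetPoint actors in the level.
; NewWave runs only once and the timer is never cleared, so spawning has no end.
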(event `self.ReceiveBeginPlay`
  (`KismetSystemLibrary.Delay` 2.0)
  (`self.NewWave`))

(event `SpawnWave`
  (`self.SpawnSpooder`))

(fn `NewWave`
  (`/Engine/EditorBlueprintResources/StandardMacros.IncrementInt` (`self.CurrentWave`)
    (:`  `
      (`KismetSystemLibrary.K2_SetTimer` null "SpawnWave" 2.0 true))))

(fn `RandomSpawnPoint`
  (returns (SpawnPoint :type "TargetPoint Object Reference"))
  (bind _outactors (`GameplayStatics.GetAllActorsOfClass` "/Script/Engine.TargetPoint"))
  (return (`|GetArrayItem` _outactors (`KismetMathLibrary.RandomIntegerInRange` 0 (`KismetArrayLibrary.Array_LastIndex` _outactors)))))

(fn `SpawnSpooder`
  (bind _spawnpoint (`self.RandomSpawnPoint`))
  (`/Engine/EditorBlueprintResources/StandardMacros.IsValid` _spawnpoint
    (:`Is Valid`
      (`|SpawnActorFromClass` "/Game/Blueprints/Pawns/BP_Spooder_01.BP_Spooder_01_C" (`self.GetTransform` _spawnpoint) "Undefined" "OverrideRootScale" null null))))

(fn `UserConstructionScript`)